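; Player Blueprint whose Fire function plays a firing montage and traces for what sits under the screen center.
; It deprojects the viewport center into the world and line-traces along that direction on the Visibility channel.
; A second trace runs from that hit location back to the mesh's transform, with no socket named.
; Both traces draw debug lines; neither applies damage or effects.
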(fn `Fire`
  (bind (_returnvalue_x _returnvalue_y) (`KismetMathLibrary.BreakVector2D` (`WidgetLayoutLibrary.GetViewportSize`)))
  (bind _returnvalue_location (`KismetMathLibrary.BreakTransform` (`SceneComponent.GetSocketTransform` (`self.Mesh`) "None" "RTS_World")))
  (bind (_worldposition _worlddirection) (`GameplayStatics.DeprojectScreenToWorld` (`GameplayStatics.GetPlayerController` 0) (`KismetMathLibrary.MakeVector2D` (/ _returnvalue_x 2.0) (/ _returnvalue_y 2.0))))
  (`self.PlayAnimMontage` "/Game/Animations/AM_Fire.AM_Fire" 1.0 "Default")
  (bind _outhit (`KismetSystemLibrary.LineTraceSingle` :`Start` _worldposition :`End` (+ _worldposition (* _worlddirection 5000.0)) :`TraceChannel` "TraceTypeQuery1" :`DrawDebugType` "ForDuration" :`DrawTime` 1.0))
  (`KismetSystemLibrary.LineTraceSingle` :`Start` (`.Location` (`GameplayStatics.BreakHitResult` _outhit)) :`End` _returnvalue_location :`TraceChannel` "TraceTypeQuery1" :`DrawDebugType` "ForDuration" :`DrawTime` 1.0))

(fn `UserConstructionScript`)